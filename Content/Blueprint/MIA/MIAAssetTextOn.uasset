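; MIAAssetTextOn is an actor that displays a tile mesh with six directional text labels around it.
; The Construction Script assigns the TileMesh variable to the static mesh and fills each label from its own text variable.
; A shared Distance offsets the labels along the local axes: Right/Left on X, Front/Back on Y, Up/Down on Z.
; The event graph holds only empty stub events, so it adds no runtime logic.
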(fn `UserConstructionScript`
  (bind _left (`self.Left`))
  (bind _front (`self.Front`))
  (bind _right (`self.Right`))
  (bind _back (`self.Back`))
  (bind _down (`self.Down`))
  (bind _up (`self.Up`))
  (`TextRenderComponent.K2_SetText` _up (`self.UpText`))
  (`SceneComponent.K2_SetRelativeLocation` _up (`KismetMathLibrary.MakeVector` 0.0 0.0 (* (`self.Distance`) 1.0)) false false)
  (`TextRenderComponent.K2_SetText` _down (`self.DownText`))
  (`SceneComponent.K2_SetRelativeLocation` _down (`KismetMathLibrary.MakeVector` 0.0 0.0 (* (`self.Distance`) -1.0)) false false)
  (`TextRenderComponent.K2_SetText` _back (`self.BackText`))
  (`SceneComponent.K2_SetRelativeLocation` _back (`KismetMathLibrary.MakeVector` 0.0 (* (`self.Distance`) -1.0)) false false)
  (`TextRenderComponent.K2_SetText` _right (`self.RightText`))
  (`SceneComponent.K2_SetRelativeLocation` _right (`KismetMathLibrary.MakeVector` (* (`self.Distance`) 1.0)) false false)
  (`TextRenderComponent.K2_SetText` _front (`self.FrontText`))
  (`SceneComponent.K2_SetRelativeLocation` _front (`KismetMathLibrary.MakeVector` 0.0 (* (`self.Distance`) 1.0)) false false)
  (`TextRenderComponent.K2_SetText` _left (`self.LeftText`))
  (`SceneComponent.K2_SetRelativeLocation` _left (`KismetMathLibrary.MakeVector` (* (`self.Distance`) -1.0)) false false)
  (`StaticMeshComponent.SetStaticMesh` (`self.StaticMesh`) (`self.TileMesh`)))